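; Game mode for a timed Moorhuhn-style shooter that starts enemy spawning, runs the countdown and handles game over.
; BeginPlay gives each BP_EnemySpawner a randomly timed SpawnEnemy timer, while a Delay on Tick counts seconds down and plays warning sounds near zero.
; At timeout it saves the player's points under a random name in a sorted top-ten save game, then shows the Highscores widget with UI-only input.
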(event `self.ReceiveBeginPlay`
  ;[1 1 1] Setup Moorhuhn spawner
  (bind _outactors (`GameplayStatics.GetAllActorsOfClass` "/Game/Blueprints/BP_EnemySpawner.BP_EnemySpawner_C"))
  (bind _output_get (set `self.EnemySpawners` _outactors))
  (for _array_element _output_get
    (`KismetSystemLibrary.K2_SetTimer` _array_element "SpawnEnemy" (`KismetMathLibrary.RandomFloatInRange` 2.0 12.0) (`self.GameRunning`))))

(event `self.ReceiveTick`
  (params (DeltaSeconds :type "Float (single-precision)"))
  (bind _returnvalue (`GameplayStatics.GetPlayerController` 0))
  (bind _scores (`/Game/Blueprints/BP_SaveGame.Scores` (`self.SaveGame`)))
  ;[1 1 1] game loop
  (`KismetSystemLibrary.Delay` 1.0)
  (if (`self.GameRunning`)
    (bind _output_get (set `self.TimeSec` (- (`self.TimeSec`) 1)))
    (if (< _output_get 1)
      (`GameplayStatics.PlaySound2D` "/Game/Audio/sfx_game_over.sfx_game_over" 1.0 1.0 0.0 null null)
      (`|ExecutionSequence`
        (:`then_0`
          (bind _asbp_fps_character (cast `/Game/Blueprints/BP_FPS_Character` (`GameplayStatics.GetPlayerCharacter` 0)))
          (set `self.PlayerPoints` (`/Game/Blueprints/BP_FPS_Character.Points` _asbp_fps_character)))
        (:`then_1`
          (`self.CreateOrLoadSaveGame`)
          (bind _output_get_2 (set `self.PlayerName` (`KismetStringLibrary.Concat_StrStr` "Player" (`KismetStringLibrary.Conv_IntToString` (`KismetMathLibrary.RandomInteger` 100)))))
          (`BlueprintMapLibrary.Map_Add` _scores _output_get_2 (`self.PlayerPoints`))
          (bind _returnvalue_2 (`Helpers.SortTopScores` _scores 10))
          (set `/Game/Blueprints/BP_SaveGame.Scores` _returnvalue_2 (`self.SaveGame`))
          (`GameplayStatics.SaveGameToSlot` (`self.SaveGame`) (`self.SaveGameSlot`))
          (bind _returnvalue_3 (`|CreateWidget` "/Game/UI/Highscores.Highscores_C" _returnvalue))
          (`UserWidget.AddToViewport` _returnvalue_3 0)
          (set `PlayerController.bShowMouseCursor` true _returnvalue)
          (`WidgetBlueprintLibrary.SetInputMode_UIOnlyEx` _returnvalue _returnvalue_3)
          (`GameplayStatics.PlaySound2D` "/Game/Audio/theme.theme" 1.0 1.0 0.0 null null)
          (set `self.GameRunning` false)))
      (elif (< _output_get 5)
        (`GameplayStatics.PlaySound2D` "/Game/Audio/sfx_time_running_out.sfx_time_running_out" 1.0 1.0 0.0 null null)))))

(fn `CreateOrLoadSaveGame`
  (bind _returnvalue (`GameplayStatics.DoesSaveGameExist` (`self.SaveGameSlot`)))
  (if _returnvalue
    (bind _returnvalue_2 (`GameplayStatics.LoadGameFromSlot` (`self.SaveGameSlot`)))
    (bind _asbp_save_game (cast `/Game/Blueprints/BP_SaveGame` _returnvalue_2)
      (:`then`
        (set `self.SaveGame` _asbp_save_game))
      (:`CastFailed`
        (bind _returnvalue_3 (`GameplayStatics.CreateSaveGameObject` "/Game/Blueprints/BP_SaveGame.BP_SaveGame_C" :!label _label))
        (set `self.SaveGame` _returnvalue_3) ; need seperate setter because only accepts one input
      ))
    (else
      (goto _label))))

(fn `UserConstructionScript`)