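; BP_Moorhuhn is a shootable chicken target that reacts when its OnHit event receives a bone and location.
; A hit plays one of three random shot sounds at the world origin and spawns an explosion emitter at the hit location.
; The mesh switches to physics simulation with a fixed impulse on the struck bone, and the actor is destroyed after a short delay.
; Body disintegration is only a TODO print.
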(event `OnHit`
  (params (Bone :type Name) (Location :type "Vector Structure"))
  (`|ExecutionSequence`
    (:`then_0`
      ;[1 1 1] Sound FX
      (switch `int` (`KismetMathLibrary.RandomInteger` 3)
        (:`0`
          (`GameplayStatics.PlaySoundAtLocation` "/Game/Audio/sfx_chicken_shot_CLOSE.sfx_chicken_shot_CLOSE" (0.0 0.0 0.0) (struct) 1.0 1.0 0.0 null null null))
        (:`1`
          (`GameplayStatics.PlaySoundAtLocation` "/Game/Audio/sfx_chicken_shot_MID.sfx_chicken_shot_MID" (0.0 0.0 0.0) (struct) 1.0 1.0 0.0 null null null))
        (:`2`
          (`GameplayStatics.PlaySoundAtLocation` "/Game/Audio/sfx_chicken_shot_FAR.sfx_chicken_shot_FAR" (0.0 0.0 0.0) (struct) 1.0 1.0 0.0 null null null))))
    (:`then_1`
      ;[1 1 1] Physics
      (`GameplayStatics.SpawnEmitterAtLocation` "/Game/Effects/SmallExplosions/P_DPW_bot_tank_explo.P_DPW_bot_tank_explo" Location)
      (`PrimitiveComponent.SetSimulatePhysics` (`self.Mesh`) true)
      (`PrimitiveComponent.AddImpulse` (`self.Mesh`) (2500.0 2500.0 0.0) Bone true)
      (`|ExecutionSequence`
        (:`then_0`
          (`KismetSystemLibrary.PrintString` "TODO: disintegrate body"))
        (:`then_1`
          (`KismetSystemLibrary.Delay` 2.0)
          (`self.K2_DestroyActor`))))))

(fn `UserConstructionScript`)