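; BP_EnemySpawner spawns BP_Moorhuhn enemies at random points inside its spawn volume when SpawnEnemy is called.
; Each spawned pawn takes the Arrow's rotation and receives its direction and score points from the spawner's variables.
; A nonzero SpawnMode is passed on as the move mode, while zero triggers a random roll that divides down to heavily favor mode 0.
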(event `SpawnEnemy`
  (bind _spawnvolume (`self.SpawnVolume`))
  ;[1 1 1] Spawn enemy within spawn volume
  (bind _returnvalue (`AIBlueprintHelperLibrary.SpawnAIFromClass` "/Game/Blueprints/BP_Moorhuhn.BP_Moorhuhn_C" null (`KismetMathLibrary.RandomPointInBoundingBox` (`SceneComponent.K2_GetComponentLocation` _spawnvolume) (`BoxComponent.GetScaledBoxExtent` _spawnvolume)) (`SceneComponent.K2_GetComponentRotation` (`self.Arrow`)) false null))
  (bind _asbp_moorhuhn (cast `/Game/Blueprints/BP_Moorhuhn` _returnvalue))
  (set `self.Moorhuhn` _asbp_moorhuhn)
  (if (== (`self.SpawnMode`) 0)
    (set `/Game/Blueprints/BP_Moorhuhn.MoveMode` (/ (`KismetMathLibrary.RandomInteger` 9) 8) (`self.Moorhuhn`))
    (else
      (set `/Game/Blueprints/BP_Moorhuhn.MoveMode` (`self.SpawnMode`) (`self.Moorhuhn`))))
  (set `/Game/Blueprints/BP_Moorhuhn.Dir` (`self.SpawnDir`) (`self.Moorhuhn`))
  (set `/Game/Blueprints/BP_Moorhuhn.ScorePoints` (`self.SpawnPoints`) (`self.Moorhuhn`)))

(fn `UserConstructionScript`)