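; BP_ScoreItem is a short-lived floating text actor, apparently a score popup, that moves and fades before destroying itself.
; BeginPlay sets the text, then the TextMove timeline lerps the TextRender's relative location between the actor's world location and that plus MoveDiff.
; TextMove's update also plays the AlphaColor timeline, which drives text alpha and destroys the actor when finished.
; A TODO notes the material's alpha channel still needs fixing.
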(event `self.ReceiveBeginPlay`
  (bind _returnvalue (`self.K2_GetActorLocation`))
  (bind (_color_r _color_g _color_b) (break `LinearColor` (`self.Color`)))
  (`self.K2_SetActorRelativeRotation` (struct :`Yaw` 180.0))
  (`TextRenderComponent.K2_SetText` (`self.TextRender`) (`self.Text`))
  (set `self.StartLocation` _returnvalue)
  (set `self.EndLocation` (+ _returnvalue (`self.MoveDiff`)))
  (bind (_direction _new_position) (`Timeline|TextMove`)
    (:`Update`
      (`SceneComponent.K2_SetRelativeLocation` (`self.TextRender`) (`KismetMathLibrary.VLerp` (`self.StartLocation`) (`self.EndLocation`) _new_position) false false)
      ;[1 1 1] TODO: fix Material -> add border and check alpha channel (color is correctly displayed in log)
      (bind (_direction_2 _alphacolor) (`Timeline|AlphaColor`)
        (:`Update`
          (`TextRenderComponent.SetTextRenderColor` (`self.TextRender`) (`KismetMathLibrary.Conv_LinearColorToColor` (`KismetMathLibrary.MakeColor` _color_r _color_g _color_b _alphacolor) false)))
        (:`Finished`
          (`self.K2_DestroyActor`))))))

(fn `UserConstructionScript`)